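; BP_OSC_Sequencer plays level sequences in response to OSC events addressed by group.
; On BeginPlay the setUniqueId graph assigns a different group ID to server and non-server instances, then enables movement replication on every DefaultPawn.
; OSCEvent accepts its own ID or a "*" wildcard, then plays the first LevelSequenceActor whose display name matches SequenceName.
; The Action argument is stored but never used.
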(event Custom|OSCEvent
  (params (group :type String) (sequenceName :type String) (action :type String))
  (Variables|Default|Setgroup group)
  (Variables|Default|SetsequenceName sequenceName)
  (Variables|Default|Setaction action)
  (if (or (Utilities|Enum|Equal(Enum) (Variables|Default|GetuniqueId) (Variables|Default|Getgroup)) (Utilities|Enum|Equal(Enum) (Variables|Default|Getgroup) "*"))
    (bind _outactors (Actor|GetAllActorsOfClass "/Script/LevelSequence.LevelSequenceActor"))
    (bind _array_element (Utilities|Array|ForEachLoopwithBreak _outactors :!label _label)
      (:LoopBody
        (if (Utilities|Enum|Equal(Enum) (Utilities|GetDisplayName _array_element) (Variables|Default|GetsequenceName))
          (bind _aslevel_sequence_actor (Utilities|Casting|CastToLevelSequenceActor _array_element)
            (:then
              (Sequencer|Player|Play (Variables|/Script/LevelSequence.LevelSequenceActor|GetSequencePlayer _aslevel_sequence_actor) :!class /Script/MovieScene.MovieSceneSequencePlayer)
              (goto _label Break))
            (:CastFailed
              (Development|PrintString "Error Casting to LevelSequenceActor")))
          (else
            (Development|PrintString (Utilities|GetDisplayName _array_element))))))
    (else
      (Development|PrintString "Msg not for me!"))))

(event EventBeginPlay
  (if (Networking|IsServer)
    (|setUniqueId :!label _label)
    (else
      (goto _label execute2))))